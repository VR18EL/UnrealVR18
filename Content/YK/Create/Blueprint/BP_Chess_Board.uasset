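; BP_Chess_Board is a chess board trigger that starts a mission when a BP_Pawn overlaps its Box.
; The overlap sets a 0.1-second timer by name for Mission_Start on the overlapping pawn, not on the board.
; The board's own Mission_Start shows the WG_PawnController widget and cursor and disables pawn input.
; Mission_End hides the cursor, removes all widgets and restores input, though it also creates an unused widget.
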(event `self.Box.OnComponentBeginOverlap`
  (params (OverlappedComponent :type "PrimitiveComponent Object Reference") (OtherActor :type "Actor Object Reference") (OtherComp :type "PrimitiveComponent Object Reference") (OtherBodyIndex :type Integer) (bFromSweep :type Boolean) (SweepResult :type "HitResult Structure (by ref)"))
  (bind _asbp_pawn (cast `/Game/YK/Create/Blueprint/BP_Pawn` OtherActor))
  (`KismetSystemLibrary.K2_SetTimer` _asbp_pawn "Mission_Start" 0.1))

(fn `Mission_End`
  (bind _returnvalue (`GameplayStatics.GetPlayerController` 0))
  (`|CreateWidget` "/Game/YK/Create/Blueprint/Widget/WG_PawnController.WG_PawnController_C" _returnvalue)
  (set `PlayerController.bShowMouseCursor` false _returnvalue)
  (`WidgetLayoutLibrary.RemoveAllWidgets`)
  (`self.EnableInput` (`GameplayStatics.GetPlayerPawn` 0) _returnvalue))

(fn `Mission_Start`
  (bind _returnvalue (`GameplayStatics.GetPlayerController` 0))
  (bind _returnvalue_2 (`|CreateWidget` "/Game/YK/Create/Blueprint/Widget/WG_PawnController.WG_PawnController_C" _returnvalue))
  (`UserWidget.AddToViewport` _returnvalue_2 0)
  (`self.DisableInput` (`GameplayStatics.GetPlayerPawn` 0) _returnvalue)
  (set `PlayerController.bShowMouseCursor` true _returnvalue))

(fn `UserConstructionScript`)