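; BP_Pawn is a chess pawn piece stepped across a board grid in a mission puzzle.
; Left, Right and UP offset the SMPawn component by fixed steps while tracking bounded XValue and YValue counters.
; Complete calls MissionEnd on BP_Chess_Board when the pawn sits on the target square, otherwise it resets position and counters.
; Controller widget and input-restoring nodes in Complete are left unconnected.
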(fn `Complete`
  (if (and (== (`self.X_Value`) 3) (== (`self.Y_Value`) 7))
    (bind _returnvalue (`GameplayStatics.GetActorOfClass` "/Game/YK/Create/Blueprint/BP_Chess_Board.BP_Chess_Board_C"))
    (`/Game/YK/Create/Blueprint/BP_Chess_Board.Mission_End` _returnvalue)
    (else
      (`SceneComponent.K2_SetRelativeLocation` (`self.SM_Pawn`) (0.0 0.0 0.0) false false)
      (set `self.Y_Value` 0)
      (set `self.X_Value` 3))))

(fn `Left`
  (if (< (`self.X_Value`) 7)
    (`SceneComponent.K2_AddLocalOffset` (`self.SM_Pawn`) (10.0 0.0 0.0) false false)
    (set `self.X_Value` (+ (`self.X_Value`) 1))))

(fn `Right`
  (if (> (`self.X_Value`) 0)
    (`SceneComponent.K2_AddLocalOffset` (`self.SM_Pawn`) (-10.0 0.0 0.0) false false)
    (set `self.X_Value` (- (`self.X_Value`) 1))))

(fn `UP`
  (bind _y_value (`self.Y_Value`))
  (if (and (<= _y_value 6) (>= _y_value 0))
    (`SceneComponent.K2_AddLocalOffset` (`self.SM_Pawn`) (0.0 10.0 0.0) false false)
    (set `self.Y_Value` (+ (`self.Y_Value`) 1))))

(fn `UserConstructionScript`)