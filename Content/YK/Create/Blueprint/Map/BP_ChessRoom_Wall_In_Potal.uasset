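; Chess room wall portal that moves the player to a fixed, hardcoded world location when its Box is overlapped.
; The construction script adds a row of hidden static mesh wall segments, evenly spaced along local X, with count driven by LoopValue and mesh by SMWall.
; The overlap event does not check which actor entered, so any overlap relocates player pawn 0 without sweeping.
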(event `self.Box.OnComponentBeginOverlap`
  (params (OverlappedComponent :type "PrimitiveComponent Object Reference") (OtherActor :type "Actor Object Reference") (OtherComp :type "PrimitiveComponent Object Reference") (OtherBodyIndex :type Integer) (bFromSweep :type Boolean) (SweepResult :type "HitResult Structure (by ref)"))
  (`self.K2_SetActorLocation` (`GameplayStatics.GetPlayerPawn` 0) (2790.0 -53.0 40.0) false false))

(fn `UserConstructionScript`
  (for _index (range (+ (`self.Loop_Value`) 1))
    (bind _returnvalue (`AddComponent|NODE_AddStaticMeshComponent-0` :`RelativeTransform` (`KismetMathLibrary.MakeTransform` (`KismetMathLibrary.MakeVector` (`KismetMathLibrary.Conv_IntToDouble` (* _index 210))))))
    (`StaticMeshComponent.SetStaticMesh` _returnvalue (`self.SM_Wall`))
    (`SceneComponent.SetVisibility` _returnvalue false false)))