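; BP_Gear_Puzzle is a gear puzzle actor with Outline, Midle and Inside components that react to hits.
; Hitting Outline turns it 45 degrees on local yaw through the OutlineGear function, while hitting Midle turns both Midle and Outline by that step.
; Hitting Inside steps through all three from inside out with short delays, but its rotation deltas are zero, so nothing turns.
; No solved-state check is present.
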(event `self.Outline.OnComponentHit`
  (params (HitComponent :type "PrimitiveComponent Object Reference") (OtherActor :type "Actor Object Reference") (OtherComp :type "PrimitiveComponent Object Reference") (NormalImpulse :type "Vector Structure") (Hit :type "HitResult Structure (by ref)"))
  (`self.Outline_Gear`))

(event `self.Midle.OnComponentHit`
  (params (HitComponent :type "PrimitiveComponent Object Reference") (OtherActor :type "Actor Object Reference") (OtherComp :type "PrimitiveComponent Object Reference") (NormalImpulse :type "Vector Structure") (Hit :type "HitResult Structure (by ref)"))
  (`SceneComponent.K2_AddLocalRotation` (`self.Midle`) (struct :`Yaw` 45.0) false false)
  (`SceneComponent.K2_AddLocalRotation` (`self.Outline`) (struct :`Yaw` 45.0) false false))

(event `self.Inside.OnComponentHit`
  (params (HitComponent :type "PrimitiveComponent Object Reference") (OtherActor :type "Actor Object Reference") (OtherComp :type "PrimitiveComponent Object Reference") (NormalImpulse :type "Vector Structure") (Hit :type "HitResult Structure (by ref)"))
  (`SceneComponent.K2_AddLocalRotation` :`self` (`self.Inside`))
  (`KismetSystemLibrary.Delay` 0.2)
  (`SceneComponent.K2_AddLocalRotation` :`self` (`self.Midle`))
  (`KismetSystemLibrary.Delay` 0.2)
  (`SceneComponent.K2_AddLocalRotation` :`self` (`self.Outline`)))

(event `self.ReceiveBeginPlay`)

(fn `Outline_Gear`
  (`SceneComponent.K2_AddLocalRotation` (`self.Outline`) (struct :`Yaw` 45.0) false false))

(fn `UserConstructionScript`)