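; Chess room gear puzzle in which three rings are rotated into alignment to open the chess room door.
; VR pawn trace hits drive stepped ring rotation, which clears that ring's aligned flag.
; Overlaps between each ring's trigger and its matching pin set the flags.
; When all three are set, it calls the door's open event, moves pin and rings through nested timelines, then destroys the puzzle after a delay.
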(event `self.ReceiveTick`
  (params (DeltaSeconds :type "Float (single-precision)")))

(event `self.ReceiveBeginPlay`
  (bind _asvrpawn_yk (cast `/Game/YK/VRPawnYK` (`GameplayStatics.GetPlayerPawn` 0)))
  (add `/Game/YK/VRPawnYK.TraceHit` _asvrpawn_yk (`|CreateDelegate` :!event `Puzzle_exe`)))

(event `self.Mat_Out.OnComponentBeginOverlap`
  (params (OverlappedComponent :type "PrimitiveComponent Object Reference") (OtherActor :type "Actor Object Reference") (OtherComp :type "PrimitiveComponent Object Reference") (OtherBodyIndex :type Integer) (bFromSweep :type Boolean) (SweepResult :type "HitResult Structure (by ref)"))
  (if (== OtherComp (`self.Out_Pin`))
    (bind _output_get (set `self.bPin_Out` true))
    (if (and _output_get (stale `self.Mat_Mid.OnComponentBeginOverlap` _output_get) (stale `self.Mat_In.OnComponentBeginOverlap` _output_get)) :!label _label
      (`self.Clear`) ; Opne Door
      (bind (_direction _newtrack_0) (`Timeline|Timeline`)
        (:`Update`
          (`SceneComponent.K2_AddWorldOffset` (`self.Pin`) (`KismetMathLibrary.MakeVector` (.y _newtrack_0) 0.0 (.y _newtrack_0)) false false)
          (bind (_direction_2 _newtrack_0_2) (`Timeline|Timeline_0`)
            (:`Update`
              (`SceneComponent.K2_AddWorldOffset` (`self.Outline`) (`KismetMathLibrary.MakeVector` 0.0 (.x _newtrack_0_2) (.y _newtrack_0_2)) false false)
              (bind (_direction_3 _newtrack_0_3) (`Timeline|Timeline_1`)
                (:`Update`
                  (`SceneComponent.K2_AddWorldOffset` (`self.Midle`) (`KismetMathLibrary.MakeVector` 0.0 (.x _newtrack_0_3) (.y _newtrack_0_3)) false false)
                  (bind (_direction_4 _newtrack_0_4) (`Timeline|Timeline_4`)
                    (:`Update`
                      (`SceneComponent.K2_AddWorldOffset` (`self.Inside`) (`KismetMathLibrary.MakeVector` 0.0 (.x _newtrack_0_4) (.y _newtrack_0_4)) false false)
                      (`KismetSystemLibrary.Delay` 4.0)
                      (bind _returnvalue (`GameplayStatics.GetActorOfClass` "BP_ChessRoom_Gear_Puzzle_C"))
                      (`self.K2_DestroyActor` _returnvalue))))))))))))

(event `self.Mat_Mid.OnComponentBeginOverlap`
  (params (OverlappedComponent :type "PrimitiveComponent Object Reference") (OtherActor :type "Actor Object Reference") (OtherComp :type "PrimitiveComponent Object Reference") (OtherBodyIndex :type Integer) (bFromSweep :type Boolean) (SweepResult :type "HitResult Structure (by ref)"))
  (if (== OtherComp (`self.Mid_Pin`))
    (bind _output_get (set `self.bPin_Mid` true))
    (goto _label)))

(event `self.Mat_In.OnComponentBeginOverlap`
  (params (OverlappedComponent :type "PrimitiveComponent Object Reference") (OtherActor :type "Actor Object Reference") (OtherComp :type "PrimitiveComponent Object Reference") (OtherBodyIndex :type Integer) (bFromSweep :type Boolean) (SweepResult :type "HitResult Structure (by ref)"))
  (if (== OtherComp (`self.In_Pin`))
    (bind _output_get (set `self.bPin_In` true))
    (goto _label)))

(fn `Clear`
  (bind _returnvalue (`GameplayStatics.GetActorOfClass` "/Game/YK/Create/Blueprint/BP_CheesRoomDoor.BP_CheesRoomDoor_C"))
  (`/Game/YK/Create/Blueprint/BP_CheesRoomDoor.Evt_Open_Call` _returnvalue))

(fn `In_Rotation`
  (params (In :type "PrimitiveComponent Object Reference"))
  (if (== In (`self.Inside`))
    (set `self.bPin_In` false)
    (if (<= (`self.Inside_Value`) 7)
      (`SceneComponent.K2_AddLocalRotation` (`self.Inside`) (struct :`Yaw` 45.0) false false)
      (set `self.Inside_Value` (+ (`self.Inside_Value`) 1))
      (else
        (bind _output_get (set `self.Inside_Value` 0))
        (`SceneComponent.K2_AddLocalRotation` (`self.Inside`) (struct :`Yaw` 45.0) false false)
        (set `self.Inside_Value` (+ _output_get 1))))
    (else
      (return))))

(fn `Mid_Rotation`
  (params (Midle :type "PrimitiveComponent Object Reference"))
  (if (== Midle (`self.Midle`))
    (set `self.bPin_Mid` false)
    (if (<= (`self.Midle_Value`) 7)
      (`SceneComponent.K2_AddLocalRotation` (`self.Midle`) (struct :`Yaw` 45.0) false false)
      (set `self.Midle_Value` (+ (`self.Midle_Value`) 1))
      (else
        (bind _output_get (set `self.Midle_Value` 0))
        (`SceneComponent.K2_AddLocalRotation` (`self.Midle`) (struct :`Yaw` 45.0) false false)
        (set `self.Midle_Value` (+ _output_get 1))))
    (else
      (return))))

(fn `Out_Rotation`
  (params (Out :type "PrimitiveComponent Object Reference"))
  (if (== Out (`self.Outline`))
    (set `self.bPin_Out` false)
    (if (<= (`self.Outline_Value`) 7)
      (`SceneComponent.K2_AddLocalRotation` (`self.Outline`) (struct :`Yaw` 45.0) false false)
      (set `self.Outline_Value` (+ (`self.Outline_Value`) 1))
      (else
        (bind _output_get (set `self.Outline_Value` 0))
        (`SceneComponent.K2_AddLocalRotation` (`self.Outline`) (struct :`Yaw` 45.0) false false)
        (set `self.Outline_Value` (+ _output_get 1))))
    (else
      (return))))

(fn `Puzzle_exe`
  (params (Hit :type "HitResult Structure"))
  (bind (_bblockinghit _binitialoverlap _time _distance _location _impactpoint _normal _impactnormal _physmat _hitactor _hitcomponent) (`GameplayStatics.BreakHitResult` Hit))
  (if (== _hitactor self)
    (`self.Out_Rotation` _hitcomponent)
    (`self.Mid_Rotation` _hitcomponent)
    (`self.In_Rotation` _hitcomponent)))

(fn `UserConstructionScript`)