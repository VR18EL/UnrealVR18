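; BP_ChessRoom_Board is the board for a chess room mission, detecting when its referenced Pawn actor enters its Box trigger.
; On overlap it swaps that actor for a new BP_ChessRoom_Pawn at a hardcoded world position with physics off, then spawns BP_ChessRoom_Move_Widget beside it.
; MissionEnd destroys the pawn found by class, plays the Seq_C_Door level sequence, then destroys the board, also found by class.
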(event `self.Box.OnComponentBeginOverlap`
  (params (OverlappedComponent :type "PrimitiveComponent Object Reference") (OtherActor :type "Actor Object Reference") (OtherComp :type "PrimitiveComponent Object Reference") (OtherBodyIndex :type Integer) (bFromSweep :type Boolean) (SweepResult :type "HitResult Structure (by ref)"))
  (bind _pawn (`self.Pawn`))
  (if (== OtherActor _pawn)
    (`self.K2_DestroyActor` _pawn)
    (bind _returnvalue (`|SpawnActorFromClass` "/Game/YK/Create/Blueprint/Mission/BP_ChessRoom_Pawn.BP_ChessRoom_Pawn_C" (`KismetMathLibrary.MakeTransform` (720.0 -245.0 124.5) (struct :`Roll` -90.0)) "Undefined" "MultiplyWithRoot" null null))
    (`PrimitiveComponent.SetSimulatePhysics` (`/Game/YK/Create/Blueprint/Mission/BP_ChessRoom_Pawn.SM_Pawn` _returnvalue) false)
    (`|SpawnActorFromClass` "/Game/YK/Create/Blueprint/BP_ChessRoom_Move_Widget.BP_ChessRoom_Move_Widget_C" (`KismetMathLibrary.MakeTransform` (645.0 -300.0 135.0) (struct)) "Undefined" "MultiplyWithRoot" null null)))

(fn `Mission_End`
  (bind _returnvalue (`GameplayStatics.GetActorOfClass` "/Game/YK/Create/Blueprint/Mission/BP_ChessRoom_Pawn.BP_ChessRoom_Pawn_C"))
  (`self.K2_DestroyActor` _returnvalue)
  (bind _outactor (`LevelSequencePlayer.CreateLevelSequencePlayer` "/Game/YK/Create/Sequence/Seq_C_Door.Seq_C_Door"))
  (`MovieSceneSequencePlayer.Play` (`LevelSequenceActor.SequencePlayer` _outactor))
  (bind _returnvalue_2 (`GameplayStatics.GetActorOfClass` "BP_ChessRoom_Board_C"))
  (`self.K2_DestroyActor` _returnvalue_2))

(fn `UserConstructionScript`)