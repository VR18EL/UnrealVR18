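; BP_Switch is a switch that toggles a referenced point light when the VR pawn's line trace hits it.
; On BeginPlay it binds to the VRPawnDK line-trace dispatcher.
; Two handler variants toggle any hit BP_Switch, not specifically themselves; the HitActor variant also fires the EDIsOn dispatcher.
; TurnOnOFF flips IsOn and sets light intensity inversely, so IsOn true means the light is dark.
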(event `self.ReceiveBeginPlay`
  (bind _asvrpawn_dk (cast `/Game/DK/Blueprints/VRPawnDK` (`GameplayStatics.GetPlayerPawn` 0)))
  (add `/Game/DK/Blueprints/VRPawnDK.ED_Linetrace` _asvrpawn_dk (`|CreateDelegate` :!event `LinetraceHitEvent2`)))

(fn `LinetraceHitEvent`
  (params (NewParam :type "Actor Object Reference"))
  (bind _asbp_switch (cast `/Game/DK/Blueprints/BP_Switch` NewParam))
  (`self.TurnOnOFF` _asbp_switch))

(fn `LinetraceHitEvent2`
  (params (NewParam :type "HitResult Structure"))
  (bind _asbp_switch (cast `/Game/DK/Blueprints/BP_Switch` (`.HitActor` (`GameplayStatics.BreakHitResult` NewParam))))
  (`self.TurnOnOFF` _asbp_switch)
  (`self.ED_IsOn`))

(fn `TurnOnOFF`
  (bind _pointlightcomponent (`PointLight.PointLightComponent` (`self.Light`)))
  (bind _output_get (set `self.bIsOn` (not (`self.bIsOn`))))
  (if _output_get
    (`LightComponent.SetIntensity` _pointlightcomponent 0.0)
    (else
      (`LightComponent.SetIntensity` _pointlightcomponent 1.0))))

(fn `UserConstructionScript`)