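; BP_Decal is a VR teleport spot whose decal marker appears on begin overlap and hides on end overlap.
; At BeginPlay it hides the decal and turns on the VRPawnDK's select line trace.
; OnLineTraceClick moves the pawn to the Box's X and Y, keeping its height and rotation.
; It then re-enables the select line trace and hides the decal.
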(event `self.ReceiveBeginPlay`
  (`SceneComponent.SetVisibility` (`self.Decal`) false false)
  (bind _asvrpawn_dk (cast `/Game/DK/Blueprints/VRPawnDK` (`GameplayStatics.GetPlayerPawn` 0)))
  (`/Game/DK/Blueprints/VRPawnDK.SetSelectLineTrace` _asvrpawn_dk true))

(fn `OnBeginOverlap`
  (`SceneComponent.SetVisibility` (`self.Decal`) true false))

(fn `OnEndOverlap`
  (`SceneComponent.SetVisibility` (`self.Decal`) false false))

(fn `OnLineTraceClick`
  (bind (_returnvalue_x _returnvalue_y) (`KismetMathLibrary.BreakVector` (`SceneComponent.K2_GetComponentLocation` (`self.Box`))))
  (bind _asvrpawn_dk (cast `/Game/DK/Blueprints/VRPawnDK` (`GameplayStatics.GetPlayerPawn` 0)))
  (bind (_returnvalue_x_2 _returnvalue_y_2 _returnvalue_z) (`KismetMathLibrary.BreakVector` (`self.K2_GetActorLocation` _asvrpawn_dk)))
  (`self.K2_SetActorLocationAndRotation` _asvrpawn_dk (`KismetMathLibrary.MakeVector` _returnvalue_x _returnvalue_y _returnvalue_z) (`self.K2_GetActorRotation` _asvrpawn_dk) false false)
  (`/Game/DK/Blueprints/VRPawnDK.SetSelectLineTrace` _asvrpawn_dk true)
  (`SceneComponent.SetVisibility` (`self.Decal`) false false))

(fn `UserConstructionScript`)