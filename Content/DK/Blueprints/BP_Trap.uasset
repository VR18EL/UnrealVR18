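; BP_Trap is a trap that launches a projectile at the player, then restarts or moves play to the DKRoom level.
; When a VRPawnDK stops overlapping the Box, a Timeline lerps the Projectile from its current location toward the player pawn each update.
; The same update chain, after short delays, fades the camera to red and opens DKRoom.
; A debug "Hello" prints on every end overlap.
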(event `self.Box.OnComponentEndOverlap`
  (params (OverlappedComponent :type "PrimitiveComponent Object Reference") (OtherActor :type "Actor Object Reference") (OtherComp :type "PrimitiveComponent Object Reference") (OtherBodyIndex :type Integer))
  (`KismetSystemLibrary.PrintString` "Hello")
  (if (== (`GameplayStatics.GetObjectClass` OtherActor) "/Game/DK/Blueprints/VRPawnDK.VRPawnDK_C")
    (bind (_direction _newtrack_0) (`Timeline|Timeline`)
      (:`Update`
        (`self.K2_SetActorLocation` (`self.Projectile`) (`KismetMathLibrary.VLerp` (`self.K2_GetActorLocation` (`self.Projectile`)) (`self.K2_GetActorLocation` (`GameplayStatics.GetPlayerPawn` 0)) _newtrack_0) false false)
        (`KismetSystemLibrary.Delay` 0.5)
        (`PlayerCameraManager.StartCameraFade` (`GameplayStatics.GetPlayerCameraManager` 0) 0.0 1.0 2.0 (struct :`R` 1.0 :`B` 0.10567 :`A` 1.0) false false)
        (`KismetSystemLibrary.Delay` 2.0)
        (`GameplayStatics.OpenLevel` "DKRoom")))))

(fn `UserConstructionScript`)