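; BP_Grab_Key_a is a trigger actor that reacts when a BP_Grab_Key enters its box.
; On overlap it hides the key mesh, disables its collision, moves it to a hardcoded relative location and shows it again, using short delays.
; It then spawns a BP_Grab_Letter and a BP_Grabl_Dagger at two referenced actors' root transforms.
; End overlap only casts to BP_Grab_Letter and does nothing further.
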(event `self.Box.OnComponentBeginOverlap`
  (params (OverlappedComponent :type "PrimitiveComponent Object Reference") (OtherActor :type "Actor Object Reference") (OtherComp :type "PrimitiveComponent Object Reference") (OtherBodyIndex :type Integer) (bFromSweep :type Boolean) (SweepResult :type "HitResult Structure (by ref)"))
  (bind _asbp_grab_key (cast `/Game/NI/BulePrint/BP_Grab_Key` OtherActor))
  (bind _staticmesh (`/Game/NI/BulePrint/BP_Grab_Key.StaticMesh` _asbp_grab_key))
  (`SceneComponent.SetVisibility` _staticmesh false false)
  (`PrimitiveComponent.SetCollisionEnabled` _staticmesh "NoCollision")
  (`KismetSystemLibrary.Delay` 0.5)
  (`SceneComponent.K2_SetRelativeLocation` _staticmesh (745.762839 -22.226093 127.526927) false false)
  (`KismetSystemLibrary.Delay` 0.5)
  (`SceneComponent.SetVisibility` _staticmesh true false)
  (`|SpawnActorFromClass` "/Game/NI/BulePrint/BP_Grab_Letter.BP_Grab_Letter_C" (`SceneComponent.K2_GetComponentToWorld` (`/Game/NI/BulePrint/BP_SpawnActor.DefaultSceneRoot` (`self.SpawnActor`))) "Undefined" "MultiplyWithRoot" null null)
  (`|SpawnActorFromClass` "/Game/NI/BulePrint/BP_Grabl_Dagger.BP_Grabl_Dagger_C" (`SceneComponent.K2_GetComponentToWorld` (`/Game/NI/BulePrint/BP_SpawnKnife.DefaultSceneRoot` (`self.SpawnActor_knife`))) "Undefined" "MultiplyWithRoot" null null))

(event `self.Box.OnComponentEndOverlap`
  (params (OverlappedComponent :type "PrimitiveComponent Object Reference") (OtherActor :type "Actor Object Reference") (OtherComp :type "PrimitiveComponent Object Reference") (OtherBodyIndex :type Integer))
  (cast `/Game/NI/BulePrint/BP_Grab_Letter` OtherActor))

(fn `UserConstructionScript`)