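; Grabbable dagger Blueprint that slices procedural mesh actors it hits, triggering an event sequence that ends in a level change.
; Hits pass a short timer-reset cooldown, then cut BP_ProceDuralActor meshes along the blade's right vector, pushing the physics halves apart.
; A slice also schedules the target's destruction, fires a slice dispatcher, runs BP_Gomdolli's event, and starts a red camera fade before loading InitMap.
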(event `self.SM_Dagger_1.OnComponentHit`
  (params (HitComponent :type "PrimitiveComponent Object Reference") (OtherActor :type "Actor Object Reference") (OtherComp :type "PrimitiveComponent Object Reference") (NormalImpulse :type "Vector Structure") (Hit :type "HitResult Structure (by ref)"))
  (if (`self.IsCanSlice`)
    (`self.SetCanSlice`)
    (`self.DoSlice` OtherActor OtherComp Hit)))

(event `self.ReceiveBeginPlay`
  (`GameplayStatics.PlaySoundAtLocation` "/Engine/EngineSounds/1kSineTonePing.1kSineTonePing" (`SceneComponent.K2_GetComponentLocation` (`self.SM_Dagger_1`)) (struct) 1.0 1.0 0.0 null null null null))

(fn `DoSlice`
  (params (HitActor :type "Actor Object Reference") (HitComponent :type "PrimitiveComponent Object Reference") (HitResult :type "HitResult Structure"))
  (bind _returnvalue (`SceneComponent.GetRightVector` (`self.SM_Dagger_1`)))
  (bind _asbp_proce_dural_actor (cast `/Game/NI/BulePrint/BP_ProceDuralActor` HitActor))
  (`/Game/NI/BulePrint/BP_ProceDuralActor.SetTimeDestroy` _asbp_proce_dural_actor 2.0)
  (bind _asprocedural_mesh_component (cast `ProceduralMeshComponent` HitComponent))
  (bind _outotherhalfprocmesh (`KismetProceduralMeshLibrary.SliceProceduralMesh` _asprocedural_mesh_component (`.Location` (`GameplayStatics.BreakHitResult` HitResult)) (`SceneComponent.GetRightVector` (`self.SM_Dagger_1`)) true "CreateNewSectionForCap" "/Game/NI/EF_MollyGreg/Common/Materials/SolidColor/BlueLightMatte_Mat.BlueLightMatte_Mat"))
  (`PrimitiveComponent.SetSimulatePhysics` _outotherhalfprocmesh true)
  (`PrimitiveComponent.SetEnableGravity` _outotherhalfprocmesh true)
  (`PrimitiveComponent.AddImpulse` _outotherhalfprocmesh (* _returnvalue 100.0) "None" false)
  (`PrimitiveComponent.AddImpulse` _asprocedural_mesh_component (* _returnvalue -100.0) "None" false)
  (`self.NewEventDispatcher_Slice` (`local.HitActor`))
  (bind _returnvalue_2 (`GameplayStatics.GetActorOfClass` "/Game/NI/BulePrint/BP_Gomdolli.BP_Gomdolli_C"))
  (`/Game/NI/BulePrint/BP_Gomdolli.Evt_Run` _returnvalue_2)
  (`PlayerCameraManager.StartCameraFade` (`GameplayStatics.GetPlayerCameraManager` 0) 0.0 1.0 10.0 (struct :`R` 1.0 :`B` 0.10567 :`A` 1.0) false false)
  (`KismetSystemLibrary.K2_SetTimer` null "MoveLevel" 10.0))

(fn `MoveLevel`
  (`GameplayStatics.OpenLevel` "InitMap"))

(fn `ResetCanSlice`
  (set `self.IsCanSlice` true))

(fn `SetCanSlice`
  (set `self.IsCanSlice` false)
  (`KismetSystemLibrary.K2_SetTimer` null "ResetCanSlice" 0.1))

(fn `UserConstructionScript`)