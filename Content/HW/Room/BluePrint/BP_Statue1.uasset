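; BP_Statue1 is a statue actor that presents a quest when the VR player's line trace hits it.
; On BeginPlay it casts the player pawn to VRPawnHW_linetrace and binds to its line trace event dispatcher.
; When the reported hit actor is itself, it spawns a BP_First_Quest_Actor at a world-space offset and sets its widget text from Quest.
; Each qualifying hit spawns a new quest actor, with no duplicate check.
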(event `self.ReceiveBeginPlay`
  (bind _asvrpawn_hw_linetrace (cast `/Game/HW/Blueprints/VRPawnHW_linetrace` (`GameplayStatics.GetPlayerPawn` 0)))
  (add `/Game/HW/Blueprints/VRPawnHW_linetrace.ED_Linetrace` _asvrpawn_hw_linetrace (`|CreateDelegate` :!event `BP_Statue_AutoGenFunc`)))

(fn `BP_Statue_AutoGenFunc`
  (params (NewParam :type "HitResult Structure"))
  (if (== (`.HitActor` (`GameplayStatics.BreakHitResult` NewParam)) self)
    (`self.ShowWidget`)))

(fn `ShowWidget`
  (bind (_returnvalue_location _returnvalue_rotation) (`KismetMathLibrary.BreakTransform` (`self.GetTransform`)))
  (bind _returnvalue (`|SpawnActorFromClass` "/Game/HW/Room/Widget/BP_First_Quest_Actor.BP_First_Quest_Actor_C" (`KismetMathLibrary.MakeTransform` (+ (30.0 0.0 100.0) _returnvalue_location) _returnvalue_rotation) "Undefined" "MultiplyWithRoot" null null))
  (`/Game/HW/Room/Widget/BP_First_Quest_Actor.WidgetTextChange` _returnvalue (`self.Quest`)))

(fn `UserConstructionScript`)