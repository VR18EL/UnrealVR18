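; BP_Pillar is a room pillar actor that shows a quest by spawning a BP_First_Quest_Actor when play begins.
; ShowWidget spawns it at the pillar's location plus a QuestLocation offset, with the pillar's rotation, then passes Quest to its WidgetTextChange.
; A handler also calls ShowWidget when a hit result matches this pillar, but the nodes binding to the VR pawn's line-trace event are disconnected.
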(event `self.ReceiveBeginPlay`
  (`self.ShowWidget`))

(fn `BP_Pillar_AutoGenFunc`
  (params (NewParam :type "HitResult Structure"))
  (if (== (`.HitActor` (`GameplayStatics.BreakHitResult` NewParam)) self)
    (`self.ShowWidget`)))

(fn `ShowWidget`
  (bind (_returnvalue_location _returnvalue_rotation) (`KismetMathLibrary.BreakTransform` (`self.GetTransform`)))
  (bind _returnvalue (`|SpawnActorFromClass` "/Game/HW/Room/Widget/BP_First_Quest_Actor.BP_First_Quest_Actor_C" (`KismetMathLibrary.MakeTransform` (+ (`self.QuestLocation`) _returnvalue_location) _returnvalue_rotation) "AlwaysSpawn" "MultiplyWithRoot" null null))
  (`/Game/HW/Room/Widget/BP_First_Quest_Actor.WidgetTextChange` _returnvalue (`self.Quest`)))

(fn `UserConstructionScript`)