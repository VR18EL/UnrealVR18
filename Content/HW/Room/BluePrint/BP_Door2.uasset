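; BP_Door2 is a room prop built from the SMChest02a and SMChest02b meshes that swings open and is revealed by a two-chest condition.
; On BeginPlay, DoOpenDoor plays a timeline that rolls SMChest02b to -90 degrees, and DoCloseDoor reverses it.
; Tick polls IsInBox on OrnateChestYellow and OrnateChestGray, making both meshes visible when both are true, with no path to hide them again.
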(event `self.ReceiveBeginPlay`
  (`self.DoOpenDoor`))

(event `DoOpenDoor`
  (bind (_direction _rotationx) (`Timeline|Timeline` :!via `PlayFromStart` :!label _label)
    (:`Update`
      (`SceneComponent.K2_SetRelativeRotation` (`self.SM_Chest_02b`) (`KismetMathLibrary.MakeRotator` (* _rotationx -90.0)) false false))))

(event `DoCloseDoor`
  (goto _label :!via `ReverseFromEnd`))

(event `self.ReceiveTick`
  (params (DeltaSeconds :type "Float (single-precision)"))
  (if (and (`/Game/HW/Room/BluePrint/BP_OrnateChest_Yellow.IsInBox` (`self.OrnateChestYellow`)) (`/Game/HW/Room/BluePrint/BP_OrnateChest_Gray.IsInBox` (`self.OrnateChestGray`)))
    (`SceneComponent.SetVisibility` (`self.SM_Chest_02b`) true false)
    (`SceneComponent.SetVisibility` (`self.SM_Chest_02a`) true false)))

(fn `UserConstructionScript`)