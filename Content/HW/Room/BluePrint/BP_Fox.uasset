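; BP_Fox is a grabbable fox room actor that reacts to its matching card, BP_Card_05_Fox.
; When that card overlaps its Box, it sets the Box's scale to half size and flags ScaleDown; other actors trigger a debug print.
; ShowWidget spawns a BP_First_Quest_Actor at an offset and passes it the Quest text, but its only call and the mesh-shrinking logic are disconnected.
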(event `self.GrabComponent.OnDropped`)

(event `self.Box.OnComponentBeginOverlap`
  (params (OverlappedComponent :type "PrimitiveComponent Object Reference") (OtherActor :type "Actor Object Reference") (OtherComp :type "PrimitiveComponent Object Reference") (OtherBodyIndex :type Integer) (bFromSweep :type Boolean) (SweepResult :type "HitResult Structure (by ref)"))
  (if (== (`GameplayStatics.GetObjectClass` OtherActor) "/Game/HW/Room/BluePrint/BP_Card_05_Fox.BP_Card_05_Fox_C")
    (`SceneComponent.SetRelativeScale3D` (`self.Box`) (0.5 0.5 0.5))
    (set `self.ScaleDown` true)
    (else
      (`KismetSystemLibrary.PrintString` "Pie"))))

(fn `ShowWidget`
  (bind (_returnvalue_location _returnvalue_rotation) (`KismetMathLibrary.BreakTransform` (`self.GetTransform`)))
  (bind _returnvalue (`|SpawnActorFromClass` "/Game/HW/Room/Widget/BP_First_Quest_Actor.BP_First_Quest_Actor_C" (`KismetMathLibrary.MakeTransform` (+ (30.0 0.0 100.0) _returnvalue_location) _returnvalue_rotation) "Undefined" "MultiplyWithRoot" null null))
  (`/Game/HW/Room/Widget/BP_First_Quest_Actor.WidgetTextChange` _returnvalue (`self.Quest`)))

(fn `UserConstructionScript`)